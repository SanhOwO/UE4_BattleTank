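; Player-controlled tank Blueprint that handles camera look and firing.
; Left/right aim input yaws an azimuth scene component and up/down input pitches the SpringArm, keeping the two camera axes on separate components.
; BeginPlay passes the barrel and turret to the tank aiming component, which also receives the fire input.
; No turret or barrel movement is scripted in this graph.
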(event `InputAxis|瞄准方位角左右`
  (params (AxisValue :type "Float (single-precision)"))
  ;[1 1 1] 摄像头视角控制
  (`SceneComponent.K2_AddLocalRotation` (`self.方位角窗口`) (`KismetMathLibrary.MakeRotator` 0.0 0.0 AxisValue) false false))

(event `InputAxis|瞄准方位角上下`
  (params (AxisValue :type "Float (single-precision)"))
  ;[1 1 1] 摄像头视角控制
  (`SceneComponent.K2_AddLocalRotation` (`self.SpringArm`) (`KismetMathLibrary.MakeRotator` 0.0 AxisValue) false false))

(event `self.ReceiveBeginPlay`
  ;[1 1 1] 绑定炮管和炮身
  (`TankAimingCompoment.Initial` (`self.TankAimingCompoment`) (`self.Barrie`) (`self.Turret`)))

(event `InputAction|开火`
  (params (Key :type "Key Structure"))
  (:`Pressed`
    (`TankAimingCompoment.Fire` (`self.TankAimingCompoment`))))

(fn `UserConstructionScript`)